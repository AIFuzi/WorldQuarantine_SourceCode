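; Character inventory component that stores picked-up items as BP_ItemInfo objects and tracks the total carried weight.
; Adding an item copies its data and class into a new info object, merges stackable items by name, destroys the world actor and updates the weight.
; Tick prints a debug list of items and weight on screen, highlighting the chosen entry.
; A name lookup returns item counts, while CanAddToInventory is a stub returning false.
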(event EventTick
  (params (DeltaSeconds :type Float%20%28single-precision%29))
  (CallFunction|GetItemsDisplay))

(fn GetItems
  (return (Variables|Items|GetItems)))

(fn AddItemtoInventory
  (params (Item :type BP%20Item%20Actor%20Object%20Reference))
  (bind _output_get (LocalVariables|SetL_Item Item))
  (bind _returnvalue (Game|ConstructObjectfromClass "/Game/Blueprints/Items/BP_ItemInfo.BP_ItemInfo_C" _output_get (Variables|/Game/Blueprints/Items/BP_ItemActor.BP_ItemActor_C|GetItemType (LocalVariables|GetL_Item)) (Variables|/Script/WorldQuarantine.ItemActor|GetItemName (LocalVariables|GetL_Item)) (Variables|/Script/WorldQuarantine.ItemActor|GetItemWeight (LocalVariables|GetL_Item)) (Variables|/Script/WorldQuarantine.ItemActor|GetCanBeStack (LocalVariables|GetL_Item)) (Variables|/Script/WorldQuarantine.ItemActor|GetItemCount (LocalVariables|GetL_Item)) (Variables|/Script/WorldQuarantine.ItemActor|GetItemUsable (LocalVariables|GetL_Item)) (Variables|/Script/WorldQuarantine.ItemActor|GetItemEquipable (LocalVariables|GetL_Item)) (Utilities|GetClass (LocalVariables|GetL_Item))))
  (bind _output_get_2 (LocalVariables|SetL_ItemInfo _returnvalue))
  (if (.ItemFinded (CallFunction|FindStackItem _output_get_2))
    (Variables|/Script/WorldQuarantine.ItemInfo|SetItemCount (.FindItem (CallFunction|FindStackItem _output_get_2)) (+ (Variables|/Script/WorldQuarantine.ItemInfo|GetItemCount (.FindItem (CallFunction|FindStackItem _output_get_2))) (.AddedCount (CallFunction|FindStackItem _output_get_2))))
    (else
      (Utilities|Array|Add (Variables|Items|GetItems) (LocalVariables|GetL_ItemInfo))))
  (Actor|DestroyActor (LocalVariables|GetL_Item))
  (CallFunction|UpdateCurrentWeight (LocalVariables|GetL_ItemInfo) "NewEnumerator0")
  (return true))

(fn FindStackItem
  (params (Item :type BP%20Item%20Info%20Object%20Reference))
  (bind _output_get (LocalVariables|SetL_Item Item))
  (if (Variables|/Script/WorldQuarantine.ItemInfo|GetCanBeStack _output_get)
    (LocalVariables|SetL_FindedItem 0)
    (LocalVariables|SetL_CanFindedItem false)
    (LocalVariables|SetL_AddedCount 0)
    (LocalVariables|SetL_ItemIndex 0)
    (bind _array_element (Utilities|Array|ForEachLoopwithBreak (CallFunction|GetItems) :!label _label)
      (:LoopBody
        (if (Utilities|Name|Equal(Name) (Variables|/Script/WorldQuarantine.ItemInfo|GetItemName _array_element) (Variables|/Script/WorldQuarantine.ItemInfo|GetItemName (LocalVariables|GetL_Item)))
          (LocalVariables|SetL_FindedItem _array_element)
          (LocalVariables|SetL_CanFindedItem true)
          (goto _label Break)))
      (:Completed
        (return (LocalVariables|GetL_FindedItem) (LocalVariables|GetL_CanFindedItem) (Variables|/Script/WorldQuarantine.ItemInfo|GetItemCount (LocalVariables|GetL_Item)))))
    (else
      (return 0 false 0))))

(fn CanAddtoInventory
  (return false))

(fn UpdateCurrentWeight
  (params (Item :type BP%20Item%20Info%20Object%20Reference) (Selection :type E_InventoryUpdateType%20Enum :default "NewEnumerator0"))
  (LocalVariables|SetL_Item Item)
  (switch Utilities|FlowControl|Switch|SwitchonE_InventoryUpdateType Selection
    (:NewEnumerator0
      (Variables|Inventory|SetInventoryCurrentWeight (+ (Variables|Inventory|GetInventoryCurrentWeight) (Variables|/Script/WorldQuarantine.ItemInfo|GetItemWeight (LocalVariables|GetL_Item)))))
    (:NewEnumerator1
      (Variables|Inventory|SetInventoryCurrentWeight (- (Variables|Inventory|GetInventoryCurrentWeight) (Variables|/Script/WorldQuarantine.ItemInfo|GetItemWeight (LocalVariables|GetL_Item)))))))

(fn GetItemsDisplay
  (for (_array_element _array_index) (Variables|Items|GetItems)
    (CallFunction|PrintMessagetoDisplay (Utilities|String|Append (Utilities|String|ToString(Name) (Variables|/Script/WorldQuarantine.ItemInfo|GetItemName _array_element)) " x" (Utilities|String|ToString(Integer) (Variables|/Script/WorldQuarantine.ItemInfo|GetItemCount _array_element)) " w:" (Utilities|String|ToString(Float) (Variables|/Script/WorldQuarantine.ItemInfo|GetItemWeight _array_element))) (select (== _array_index (Variables|Default|GetChooseItem)) "(R=1.000000,G=0.049797,B=0.769483,A=1.000000)" "(R=0.276042,G=0.276042,B=0.276042,A=1.000000)") 0.0))
  (CallFunction|PrintMessagetoDisplay (Utilities|String|Append "Current weight+== " (Utilities|String|ToString(Float) (Variables|Inventory|GetInventoryCurrentWeight))) "(R=0.154965,G=1.000000,B=0.160009,A=1.000000)" 0.0)
  (CallFunction|PrintMessagetoDisplay "Inventory: ===" "(R=1.000000,G=0.297126,B=0.760883,A=1.000000)" 0.0))

(fn FindItemsinInventory
  (params (ItemName :type Name))
  (LocalVariables|SetL_ItemName ItemName)
  (bind (_array_element _array_index) (Utilities|Array|ForEachLoopwithBreak (Variables|Items|GetItems))
    (:LoopBody
      (if (Utilities|Name|Equal(Name) (Variables|/Script/WorldQuarantine.ItemInfo|GetItemName _array_element) (LocalVariables|GetL_ItemName))
        (LocalVariables|SetL_FindedItem true)
        (LocalVariables|SetL_Count (Variables|/Script/WorldQuarantine.ItemInfo|GetItemCount _array_element))))
    (:Completed
      (return (LocalVariables|GetL_FindedItem) _array_index (LocalVariables|GetL_Count)))))